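; Skill weapon Blueprint for the first-person player, a child class that sets its own ammo, reload time and bullet spread on construction.
; AmmoCheck decrements ammo, then plays the revolver fire animation and prints the count unless the player is reloading.
; LineTrace casts a randomly spread ray from the camera, then a second from the muzzle to that impact point.
; Both traces only draw debug lines, and a Niagara spawn is left unconnected.
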(fn `AmmoCheck`
  (`/Engine/EditorBlueprintResources/StandardMacros.DecrementInt` (`self.AmmoCount`)
    (:`  `
      (if (not (`/Game/Luke/Blueprints/FPSCharacterLuke_BP.IsReloading` (cast `/Game/Luke/Blueprints/FPSCharacterLuke_BP` (`GameplayStatics.GetPlayerCharacter` 0) :!pure true)))
        (`SkeletalMeshComponent.PlayAnimation` (`self.PrimaryWeapon`) "/Game/Luke/Animations/FPS_RevolverFire_animMontageNEW1.FPS_RevolverFire_animMontageNEW1" false)
        (`KismetSystemLibrary.PrintString` (`KismetStringLibrary.Conv_IntToString` (`self.AmmoCount`)))))))

(fn `LineTrace`
  (bind _bulletspread (`self.BulletSpread`))
  (bind _returnvalue (* _bulletspread -1.0))
  (bind _firstpersoncamera (`/Game/Luke/Blueprints/FPSCharacterLuke_BP.FirstPersonCamera` (cast `/Game/Luke/Blueprints/FPSCharacterLuke_BP` (`GameplayStatics.GetPlayerCharacter` 0) :!pure true)))
  (bind _returnvalue_2 (`SceneComponent.K2_GetComponentLocation` _firstpersoncamera))
  (bind _outhit (`KismetSystemLibrary.LineTraceSingle` :`Start` _returnvalue_2 :`End` (+ (+ (* (`SceneComponent.GetForwardVector` _firstpersoncamera) 200000.0) _returnvalue_2) (`KismetMathLibrary.MakeVector` (`KismetMathLibrary.RandomFloatInRange` _returnvalue _bulletspread) (`KismetMathLibrary.RandomFloatInRange` _returnvalue _bulletspread) (`KismetMathLibrary.RandomFloatInRange` _returnvalue _bulletspread))) :`TraceChannel` "TraceTypeQuery1" :`DrawDebugType` "ForDuration" :`TraceColor` (struct :`R` 1.0 :`G` 0.111708 :`B` 0.862471 :`A` 1.0))) ; Camera Shot
  (`KismetSystemLibrary.LineTraceSingle` :`Start` (`SceneComponent.K2_GetComponentLocation` (`self.Muzzle`)) :`End` (`.ImpactPoint` (`GameplayStatics.BreakHitResult` _outhit)) :`TraceChannel` "TraceTypeQuery1" :`DrawDebugType` "ForDuration" :`TraceColor` (struct :`R` 1.0 :`G` 0.130136 :`A` 1.0) :`TraceHitColor` (struct :`R` 1.0 :`G` 0.130136 :`A` 1.0)) ; Gun Shot
)

(fn `UserConstructionScript`
  (`parent.UserConstructionScript`)
  (set `self.MaxAmmo` 300)
  (set `self.AmmoCount` 300)
  (set `self.ReloadTime` 3.0)
  (set `self.BulletSpread` 400.0))